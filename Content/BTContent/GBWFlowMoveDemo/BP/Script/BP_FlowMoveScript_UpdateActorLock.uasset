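; Flow Move update script that gives the local player lock-on feedback for the focused actor component.
; Init and Update share one pass that creates a target widget, plays get or lost sounds on focus changes, and projects the last focus location to screen to position the widget.
; With camera lock enabled and in actor-lock view mode, control yaw interpolates toward the focus, only when the local player is also the server.
; End removes the widget.
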(event EventOnUpdate
  (params (EventType :type EGBWFlowMoveEventType%20Enum :default "Init") (NetworkLocation :type EFlowMoveNetworkLocationType%20Enum :default "Server") (bIsLocalOwn :type Boolean) (FlowMoveComponent :type GBW%20Flow%20Move%20Component%20Object%20Reference))
  (CallFunction|EventUpdate EventType NetworkLocation bIsLocalOwn FlowMoveComponent))

(fn EventUpdate
  (params (Event%20Type :type EGBWFlowMoveEventType%20Enum :default "Init") (NetworkLocation :type EFlowMoveNetworkLocationType%20Enum :default "Server") (bIsLocalOwn :type Boolean) (FlowMoveComponent :type GBW%20Flow%20Move%20Component%20Object%20Reference))
  (bind _taskstate (Variables|/Script/GBWFlowMove.GBWFlowMoveComponent|GetTaskState FlowMoveComponent))
  (bind _taskstate_2 (Variables|/Script/GBWFlowMove.GBWFlowMoveComponent|GetTaskState FlowMoveComponent))
  (bind _taskstate_3 (Variables|/Script/GBWFlowMove.GBWFlowMoveComponent|GetTaskState FlowMoveComponent))
  (bind _focusactorcomponent (Utilities|Struct|BreakGBWFlowMoveState _taskstate))
  (bind (_flowmovecomponentguid _flowmovecomponent _ownercharacter _bisactive _bisstopping _timer _framedeltatime _framenumber _movementmode _viewmode _focusactorcomponent_2) (Utilities|Struct|BreakGBWFlowMoveState _taskstate_3))
  (bind (_flowmovecomponentguid_2 _flowmovecomponent_2 _ownercharacter_2 _bisactive_2 _bisstopping_2 _timer_2 _framedeltatime_2 _framenumber_2 _movementmode_2 _viewmode_2 _focusactorcomponent_3) (Utilities|Struct|BreakGBWFlowMoveState _taskstate_2))
  (bind _returnvalue (Pawn|GetController _ownercharacter))
  (bind _returnvalue_2 (Pawn|GetControlRotation _returnvalue :!class /Script/Engine.Controller))
  (bind (_roll _pitch) (Math|Rotator|BreakRotator _returnvalue_2))
  (switch Utilities|FlowControl|Switch|SwitchonEGBWFlowMoveEventType Event%20Type
    (:Init
      (if (Class|GBWFlowMoveComponent|IsLocalPlayer FlowMoveComponent) :!label _label
        (Utilities|FlowControl|Sequence
          (:then_0
            (if (and (not (Utilities|IsValid (Variables|Runtime|GetActorTargetWidget))) (Utilities|IsValidClass (Variables|Settings|GetActorTargetWidgetClass)))
              (bind _returnvalue_3 (UserInterface|CreateWidget (Variables|Settings|GetActorTargetWidgetClass) (Pawn|GetLocalViewingPlayerController (.OwnerCharacter (Utilities|Struct|BreakGBWFlowMoveState (Variables|/Script/GBWFlowMove.GBWFlowMoveComponent|GetTaskState FlowMoveComponent))))))
              (Variables|Runtime|SetActorTargetWidget _returnvalue_3)))
          (:then_1
            (if (!= _focusactorcomponent (Variables|Runtime|GetLastFocusActorComponent))
              (if (Utilities|IsValid _focusactorcomponent)
                (Audio|PlaySound2D (Variables|Settings|GetActorGetSound) 1.0 1.0 0.0 0 0)
                (else
                  (Audio|PlaySound2D (Variables|Settings|GetActorLostSound) 1.0 1.0 0.0 0 0)))))
          (:then_2
            (Utilities|IsValid (Variables|Runtime|GetActorTargetWidget)
              (:Is%20Valid
                (Utilities|IsValid (Variables|Runtime|GetLastFocusActorComponent)
                  (:Is%20Valid
                    (if (UserInterface|Viewport|IsinViewport (Variables|Runtime|GetActorTargetWidget))
                      _
                      (else
                        (UserInterface|Viewport|AddtoViewport (Variables|Runtime|GetActorTargetWidget) 0)))
                    (if (.ReturnValue (Class|WidgetLayoutLibrary|ProjectWorldLocationtoWidgetPosition (Pawn|GetLocalViewingPlayerController (.OwnerCharacter (Utilities|Struct|BreakGBWFlowMoveState (Variables|/Script/GBWFlowMove.GBWFlowMoveComponent|GetTaskState FlowMoveComponent)))) (Transformation|GetWorldLocation (Variables|Runtime|GetLastFocusActorComponent)) false))
                      (Class|Widget|SetRenderTranslation (Variables|Runtime|GetActorTargetWidget) (.ScreenPosition (Class|WidgetLayoutLibrary|ProjectWorldLocationtoWidgetPosition (Pawn|GetLocalViewingPlayerController (.OwnerCharacter (Utilities|Struct|BreakGBWFlowMoveState (Variables|/Script/GBWFlowMove.GBWFlowMoveComponent|GetTaskState FlowMoveComponent)))) (Transformation|GetWorldLocation (Variables|Runtime|GetLastFocusActorComponent)) false)))))
                  (:Is%20Not%20Valid
                    (if (UserInterface|Viewport|IsinViewport (Variables|Runtime|GetActorTargetWidget)) :!label _label_2
                      (Widget|RemovefromParent (Variables|Runtime|GetActorTargetWidget))))))))
          (:then_3
            (if (Class|GBWFlowMoveComponent|IsinServer FlowMoveComponent)
              (if (Variables|Settings|GetUseCameraLock)
                (Utilities|IsValid _focusactorcomponent_2
                  (:Is%20Valid
                    (if (Utilities|Enum|Equal(Enum) _viewmode "TP_ActorLockMode")
                      (Pawn|SetControlRotation _returnvalue (Math|Rotator|MakeRotator _roll _pitch (.yaw (Math|Interpolation|RInterpTo _returnvalue_2 (Math|Rotator|FindLookatRotation (Transformation|GetActorLocation _ownercharacter) (Transformation|GetWorldLocation _focusactorcomponent_2)) (Utilities|Time|GetWorldDeltaSeconds) (Variables|Settings|GetCameraLockInterpSpeed)))))))))))
          (:then_4
            (Variables|Runtime|SetLastViewMode _viewmode_2)
            (Variables|Runtime|SetLastFocusActorComponent _focusactorcomponent_3)))))
    (:Update
      (goto _label))
    (:End
      (goto _label_2))))