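; FlowMove script that shows an attribute widget beside the local player's character while the task is active and for three seconds afterwards.
; On update it lazily creates the widget, then removes it from the viewport once the inactive timer expires.
; The widget eases toward a projected point right of the character through a next-tick delay loop.
; Two attributes feed percentages as value over range size, and a third feeds a number.
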(event EventOnUpdate
  (params (EventType :type EGBWFlowMoveEventType%20Enum :default "Init") (NetworkLocation :type EFlowMoveNetworkLocationType%20Enum :default "Server") (bIsLocalOwn :type Boolean) (FlowMoveComponent :type GBW%20Flow%20Move%20Component%20Object%20Reference))
  (bind _taskstate (Variables|/Script/GBWFlowMove.GBWFlowMoveComponent|GetTaskState FlowMoveComponent))
  (bind (_flowmovecomponentguid _flowmovecomponent _ownercharacter _bisactive _bisstopping _timer _framedeltatime) (Utilities|Struct|BreakGBWFlowMoveState _taskstate))
  (bind _returnvalue (Transformation|GetActorLocation _ownercharacter))
  (bind _returnvalue_2 (Pawn|GetController _ownercharacter))
  (bind _returnvalue_3 (Pawn|GetLocalViewingPlayerController _ownercharacter))
  (bind _returnvalue_4 (Transformation|GetActorRightVector _returnvalue_2))
  (bind _returnvalue_5 (* _returnvalue_4 3e+01))
  (bind _returnvalue_6 (+ _returnvalue _returnvalue_5))
  (bind (_screenposition _returnvalue_7) (Class|WidgetLayoutLibrary|ProjectWorldLocationtoWidgetPosition _returnvalue_3 _returnvalue_6 false))
  (if (Class|GBWFlowMoveComponent|IsLocalPlayer FlowMoveComponent)
    (if _bisactive
      (Variables|Runtime|SetTimer 0.0)
      (Utilities|FlowControl|Sequence :!label _label
        (:then_0
          (Utilities|IsValid (Variables|Runtime|GetUI)
            (:Is%20Valid
              (if (not (UserInterface|Viewport|IsinViewport (Variables|Runtime|GetUI)))
                (UserInterface|Viewport|AddtoViewport (Variables|Runtime|GetUI) 0 :!label _label_2)))
            (:Is%20Not%20Valid
              (bind _returnvalue_8 (UserInterface|CreateWidget "/Game/BTContent/OtherAssets/HUD/UI_FlowMoveAttribute.UI_FlowMoveAttribute_C" _returnvalue_3))
              (Variables|Runtime|SetUI _returnvalue_8)
              (goto _label_2))))
        (:then_1
          (Utilities|IsValid (Variables|Runtime|GetUI)
            (:Is%20Valid
              (Utilities|FlowControl|Sequence
                (:then_0
                  (if _returnvalue_7
                    (Variables|Runtime|SetUIScreenPosition _screenposition)
                    (Utilities|FlowControl|DelayUntilNextTick :!label _label_3)
                    (Utilities|IsValid (Variables|Runtime|GetUI)
                      (:Is%20Valid
                        (if (UserInterface|Viewport|IsinViewport (Variables|Runtime|GetUI))
                          (Class|Widget|SetRenderTranslation (Variables|Runtime|GetUI) (Class|KismetMathLibrary|Vector2DInterpto (.Translation (Utilities|Struct|BreakWidgetTransform (Variables|/Script/UMG.Widget|GetRenderTransform (Variables|Runtime|GetUI)))) (Variables|Runtime|GetUIScreenPosition) (Utilities|Time|GetWorldDeltaSeconds) 1e+01))
                          (goto _label_3))))))
                (:then_1
                  (bind (_attribute _returnvalue_9) (Class|GBWFlowMoveComponent|GetAttribute _flowmovecomponent (Variables|Settings|GetAttribute_1)))
                  (if _returnvalue_9
                    (Default|SetPercent1 (Variables|Runtime|GetUI) (/ (.Value (Utilities|Struct|Break _attribute)) (- (.Range_Max (Utilities|Struct|Break _attribute)) (.Range_Min (Utilities|Struct|Break _attribute)))))))
                (:then_2
                  (bind (_attribute_2 _returnvalue_10) (Class|GBWFlowMoveComponent|GetAttribute _flowmovecomponent (Variables|Settings|GetAttribute_2)))
                  (if _returnvalue_10
                    (Default|SetPercent2 (Variables|Runtime|GetUI) (/ (.Value (Utilities|Struct|Break _attribute_2)) (- (.Range_Max (Utilities|Struct|Break _attribute_2)) (.Range_Min (Utilities|Struct|Break _attribute_2)))))))
                (:then_3
                  (bind (_attribute_3 _returnvalue_11) (Class|GBWFlowMoveComponent|GetAttribute _flowmovecomponent (Variables|Settings|GetAttribute_3)))
                  (if _returnvalue_11
                    (Default|SetNumber1 (Variables|Runtime|GetUI) (Utilities|Struct|Break _attribute_3)))))))))
      (else
        (bind _output_get (Variables|Runtime|SetTimer (+ (Variables|Runtime|GetTimer) _framedeltatime)))
        (if (>= _output_get 3.0)
          (Utilities|IsValid (Variables|Runtime|GetUI)
            (:Is%20Valid
              (if (UserInterface|Viewport|IsinViewport (Variables|Runtime|GetUI))
                (Widget|RemovefromParent (Variables|Runtime|GetUI)))))
          (else
            (goto _label)))))))