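; FlowMove update script that drives the visuals and audio of a hook launched from the owning character toward the action's target point.
; On Init and Update it spawns a tagged Niagara ribbon at a mesh socket with a launch sound, then lerps its TailEnd to the target over the launch duration.
; Full extension triggers a one-shot impact effect and attach sound.
; End destroys the tagged ribbon components.
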(event EventOnUpdate
  (params (EventType :type EGBWFlowMoveEventType%20Enum :default "Init") (NetworkLocation :type EFlowMoveNetworkLocationType%20Enum :default "Server") (bIsLocalOwn :type Boolean) (FlowMoveComponent :type GBW%20Flow%20Move%20Component%20Object%20Reference))
  (bind _taskstate (Variables|/Script/GBWFlowMove.GBWFlowMoveComponent|GetTaskState FlowMoveComponent))
  (bind _taskstate_2 (Variables|/Script/GBWFlowMove.GBWFlowMoveComponent|GetTaskState FlowMoveComponent))
  (bind _hooktag (Variables|Settings|GetHookTag))
  (bind _ownercharacter (Utilities|Struct|BreakGBWFlowMoveState _taskstate))
  (bind (_flowmovecomponentguid _flowmovecomponent _ownercharacter_2 _bisactive _bisstopping _timer _framedeltatime) (Utilities|Struct|BreakGBWFlowMoveState _taskstate_2))
  (bind _returnvalue (Actor|GetComponentsbyTag _ownercharacter_2 "/Script/Niagara.NiagaraComponent" _hooktag))
  (bind _returnvalue_2 (Transformation|GetActorTransform _ownercharacter_2))
  (bind _mesh (Variables|/Script/Engine.Character|GetMesh _ownercharacter_2))
  (switch Utilities|FlowControl|Switch|SwitchonEGBWFlowMoveEventType EventType
    (:Init
      (Utilities|IsValid _ownercharacter_2 :!label _label
        (:Is%20Valid
          (Variables|Runtime|SetTimer (+ (Variables|Runtime|GetTimer) _framedeltatime))
          (if (Utilities|Array|IsEmpty _returnvalue)
            (bind _returnvalue_3 (Niagara|SpawnSystemAttached "/Game/BTContent/OtherAssets/NS/NS_Ribbon_Twist.NS_Ribbon_Twist" _mesh (Variables|Settings|GetAttachSlotName) "0, 0, 0" "0, 0, 0" "KeepRelativeOffset" false))
            (Utilities|IsValid _returnvalue_3
              (:Is%20Valid
                (Variables|/Script/Engine.ActorComponent|SetComponentTags _returnvalue_3 (Utilities|Array|MakeArray (Variables|Settings|GetHookTag)))
                (Effects|Components|ParticleSystem|SetVectorParameter _returnvalue_3 "TailEnd" (Transformation|GetSocketLocation _mesh (Variables|Settings|GetAttachSlotName)))
                (Variables|Runtime|SetTimer 0.0)
                (Variables|Runtime|SetHasExected false)
                (Audio|PlaySoundatLocation (Variables|Settings|GetLaunchSound) (.location _returnvalue_2) (.rotation _returnvalue_2) 1.0 1.0 0.0 0 0 0 0)))
            (else
              (for _array_element _returnvalue
                (Utilities|IsValid _array_element
                  (:Is%20Valid
                    (Effects|Components|ParticleSystem|SetVectorParameter _array_element "TailEnd" (Math|Vector|Lerp(Vector) (Transformation|GetSocketLocation _mesh (Variables|Settings|GetAttachSlotName)) (.Point (Utilities|Struct|BreakGBWFlowMovePointScene (.TargetLocationScene (Utilities|Struct|BreakGBWFlowMoveScene (.CurrentActionTargetScene (Utilities|Struct|BreakGBWFlowMoveState (.BeginFlowMoveState (Utilities|Struct|BreakGBWFlowMoveRMSControllerInitInfo (Variables|/Script/GBWFlowMove.GBWFlowMoveComponent|GetCurrentActionTargetSceneInfo FlowMoveComponent))))))))) (Math|Float|Clamp(Float) (/ (Variables|Runtime|GetTimer) (Variables|Settings|GetLaunchDuration)))))
                    (if (>= (Math|Float|Clamp(Float) (/ (Variables|Runtime|GetTimer) (Variables|Settings|GetLaunchDuration))) 1.0)
                      (if (not (Variables|Runtime|GetHasExected))
                        (Niagara|SpawnSystematLocation "/Game/BTContent/OtherAssets/NS/NS_ProjectileDie.NS_ProjectileDie" (Math|Vector|Lerp(Vector) (Transformation|GetSocketLocation _mesh (Variables|Settings|GetAttachSlotName)) (.Point (Utilities|Struct|BreakGBWFlowMovePointScene (.TargetLocationScene (Utilities|Struct|BreakGBWFlowMoveScene (.CurrentActionTargetScene (Utilities|Struct|BreakGBWFlowMoveState (.BeginFlowMoveState (Utilities|Struct|BreakGBWFlowMoveRMSControllerInitInfo (Variables|/Script/GBWFlowMove.GBWFlowMoveComponent|GetCurrentActionTargetSceneInfo FlowMoveComponent))))))))) (Math|Float|Clamp(Float) (/ (Variables|Runtime|GetTimer) (Variables|Settings|GetLaunchDuration)))) (.rotation _returnvalue_2) (.scale _returnvalue_2))
                        (Audio|PlaySoundatLocation (Variables|Settings|GetAttachSound) (.location _returnvalue_2) (.rotation _returnvalue_2) 2.0 1.0 0.0 0 0 0 0)
                        (Variables|Runtime|SetHasExected true)))))))))))
    (:Update
      (goto _label))
    (:End
      (Utilities|IsValid _ownercharacter
        (:Is%20Valid
          (for _array_element_2 (Actor|GetComponentsbyTag _ownercharacter "/Script/Niagara.NiagaraComponent" (Variables|Settings|GetHookTag))
            (Utilities|IsValid _array_element_2
              (:Is%20Valid
                (Components|DestroyComponent _array_element_2)))))))))